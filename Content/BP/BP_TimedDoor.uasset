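; BP_TimedDoor is a garage door that starts down and locked, with a red status light.
; Unlocking turns the light green and raises the folding door, while locking turns it red and lowers it.
; Separate raise and lower timelines offset the door's Z from its saved start location, updating up and down flags.
; The moving flag is never set true, and no timer or trigger appears in the graph.
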(event `self.ReceiveBeginPlay`
  (bind (_returnvalue_x _returnvalue_y _returnvalue_z) (`KismetMathLibrary.BreakVector` (`SceneComponent.K2_GetComponentLocation` (`self.foldingDoor`))))
  ;[1 1 1] Initial Set up for garage door
  ;;[1 1 1] get folding door's initial XYZ and save it
  (set `self.StartX` _returnvalue_x)
  (set `self.StartY` _returnvalue_y)
  (set `self.StartZ` _returnvalue_z)
  ;;[1 1 1] Set the initial states of door to down, not up or moving, and locked
  (set `self.doorIsDown` true)
  (set `self.doorIsUp` false)
  (set `self.doorIsMoving` false)
  (set `self.doorIsLocked` true)
  ;;[1 1 1] Set statusLight to red
  (`PrimitiveComponent.SetMaterial` (`self.statusLight`) 0 "/Game/Materials/MM_statusRed.MM_statusRed"))

(event `eventRaiseDoor`
  ;[1 1 1] Raise the door
  (set `self.doorIsDown` false)
  (bind (_direction _garagedoorheight) (`Timeline|Raise the door` :!via `PlayFromStart`)
    (:`Update`
      (`SceneComponent.K2_SetWorldLocation` (`self.foldingDoor`) (`KismetMathLibrary.MakeVector` (`self.StartX`) (`self.StartY`) (+ _garagedoorheight (`self.StartZ`))) false false))
    (:`Finished`
      (set `self.doorIsUp` true)
      (set `self.doorIsMoving` false))))

(event `eventLowerDoor`
  ;[1 1 1] Lower the door
  (set `self.doorIsUp` false)
  (bind (_direction _garagedoorheight) (`Timeline|Lower the door`)
    (:`Update`
      (`SceneComponent.K2_SetWorldLocation` (`self.foldingDoor`) (`KismetMathLibrary.MakeVector` (`self.StartX`) (`self.StartY`) (+ _garagedoorheight (`self.StartZ`))) false false))
    (:`Finished`
      (set `self.doorIsDown` true)
      (set `self.doorIsMoving` false))))

(event `eventUnlockDoor`
  ;[1 1 1] Unlock Door
  (set `self.doorIsLocked` false)
  (`PrimitiveComponent.SetMaterial` (`self.statusLight`) 0 "/Game/Materials/MM_statusGreen.MM_statusGreen")
  (`self.eventRaiseDoor`))

(event `eventLockDoor`
  ;[1 1 1] Lock Door
  (set `self.doorIsLocked` true)
  (`PrimitiveComponent.SetMaterial` (`self.statusLight`) 0 "/Game/Materials/MM_statusRed.MM_statusRed")
  (`self.eventLowerDoor`))

(fn `UserConstructionScript`)