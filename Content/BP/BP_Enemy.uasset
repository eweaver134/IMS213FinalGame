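; BP_Enemy is an enemy that wanders the navigable area and ends the game when it touches the player.
; From BeginPlay it loops AI MoveTo toward random reachable points within a radius of its current location, picking a new one only after each successful move.
; Overlapping BP_ThirdPersonCharacter destroys both the player and the enemy, then quits the game.
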(event `self.ReceiveBeginPlay`
  ;[1 1 1] Random Momenent across available area
  (`self.Random Roam`))

(event `Random Roam`
  ;[1 1 1] Random Momenent across available area
  (`|AIMoveTo` self (`NavigationSystemV1.K2_GetRandomReachablePointInRadius` (`self.K2_GetActorLocation`) 2500.0 null null) null
    (:`OnSuccess`
      (`self.Random Roam`))))

(event `self.ReceiveActorBeginOverlap`
  (params (OtherActor :type "Actor Object Reference"))
  ;[1 1 1] Destroys Player and Enemy on collision then ends game
  (bind _asbp_third_person_character (cast `/Game/ThirdPerson/Blueprints/BP_ThirdPersonCharacter` OtherActor))
  (`self.K2_DestroyActor` _asbp_third_person_character)
  (`self.K2_DestroyActor`)
  (`KismetSystemLibrary.QuitGame` null "Quit"))

(fn `UserConstructionScript`)